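; Game mode for the Guards gameplay that handles game over and restarts the current level.
; TriggerGameOver runs only once via an IsGameOver flag, fires the OnGameOver dispatcher and shows a WBP_GameOver widget.
; It then disables player pawn input, waits RestartDelay and reloads the current level by name.
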(event Custom|TriggerGameOver
  (bind _returnvalue (Game|GetPlayerController 0))
  (if (not (Variables|GameOver|GetbIsGameOver))
    (Variables|GameOver|SetbIsGameOver true)
    (Default|CallOnGameOver)
    (bind _returnvalue_2 (UserInterface|CreateWidget "/Game/Guards/UI/WBP_GameOver.WBP_GameOver_C" _returnvalue))
    (UserInterface|Viewport|AddtoViewport _returnvalue_2 0)
    (Input|DisableInput (Game|Player|GetPlayerPawn 0) _returnvalue)
    (Utilities|FlowControl|Delay (Variables|GameOver|GetRestartDelay))
    (bind _returnvalue_3 (Game|GetCurrentLevelName true))
    (Game|OpenLevel(byName) (Utilities|String|StringToName _returnvalue_3))))

(event EventBeginPlay)

(event EventTick
  (params (DeltaSeconds :type Float%20%28single-precision%29)))

(fn ConstructionScript
  (|CallParentFunction))
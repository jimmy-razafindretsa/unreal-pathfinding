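; BP_Guard is an enemy guard that switches between passive, chase and search alert modes and ends the game when it catches the player.
; Each mode event calls ApplyAlertMode, which sets the walk speed and updates the label and tint on its WBP_GuardState widget.
; An overlap of CatchSphere with the player pawn triggers game over through BP_GuardGameMode.
; The file holds no logic that decides when modes change.
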(event OnComponentBeginOverlap(CatchSphere)
  (params (OverlappedComponent :type Primitive%20Component%20Object%20Reference) (OtherActor :type Actor%20Object%20Reference) (OtherComp :type Primitive%20Component%20Object%20Reference) (OtherBodyIndex :type Integer) (bFromSweep :type Boolean) (SweepResult :type Hit%20Result%20Structure%20%28by%20ref%29))
  (if (== OtherActor (Game|Player|GetPlayerPawn 0))
    (bind _asbp_guard_game_mode (Utilities|Casting|CastToBP_GuardGameMode (Game|GetGameMode)))
    (Default|TriggerGameOver _asbp_guard_game_mode)))

(event Custom|EnterPassive
  (CallFunction|ApplyAlertMode (Variables|Guard|GetPatrolSpeed) "PASSIF" "(R=0.200000,G=0.900000,B=0.300000,A=1.000000)"))

(event Custom|EnterChase
  (CallFunction|ApplyAlertMode (Variables|Guard|GetChaseSpeed) "EN CHASSE" "(R=1.000000,G=0.150000,B=0.100000,A=1.000000)"))

(event Custom|EnterSearch
  (CallFunction|ApplyAlertMode (Variables|Guard|GetSearchSpeed) "RECHERCHE" "(R=1.000000,G=0.650000,B=0.050000,A=1.000000)"))

(fn ConstructionScript)

(fn ApplyAlertMode
  (params (Speed :type Float%20%28double-precision%29) (Label :type Text) (Tint :type Linear%20Color%20Structure))
  (Variables|/Script/Engine.CharacterMovementComponent|SetMaxWalkSpeed (Variables|Character|GetCharacterMovement) Speed)
  (bind _aswbp_guard_state (Utilities|Casting|CastToWBP_GuardState (UserInterface|GetUserWidgetObject (Variables|Default|GetStateWidget))))
  (Default|SetDisplayedState _aswbp_guard_state Label Tint))
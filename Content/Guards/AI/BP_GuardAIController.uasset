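; AI controller for guards that patrol, chase the player on sight or other perception, and search after losing them.
; Boolean flags select the state, and move-completed results drive the next step: re-chase, timed search or next looping checkpoint, with retries on failed patrol moves.
; Perception updates switch between chasing and searching the last known location, notifying the Guard pawn of each mode.
; The game mode's game-over event halts movement.
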(event OnTargetPerceptionUpdated(Perception)
  (params (Actor :type Actor%20Object%20Reference) (Stimulus :type AI%20Stimulus%20Structure))
  (bind (_age _expirationage _strength _stimuluslocation _receiverlocation _tag _bsuccessfullysensed) (Utilities|Struct|BreakAIStimulus Stimulus))
  (if (== Actor (Game|Player|GetPlayerPawn 0))
    (if _bsuccessfullysensed
      (Variables|GuardAI|SetChaseTarget Actor)
      (CallFunction|StartChase)
      (else
        (Variables|GuardAI|SetLastKnownLocation _stimuluslocation)
        (CallFunction|LoseTarget)))))

(event Custom|MoveToCurrentCheckpoint
  (bind _guard (Variables|GuardAI|GetGuard))
  (bind _checkpointindex (Variables|GuardAI|GetCheckpointIndex))
  (bind _patrolpath (Variables|/Game/Guards/Characters/BP_Guard.BP_Guard_C|GetPatrolPath _guard))
  (bind _checkpoints (Variables|/Game/Guards/Gameplay/BP_PatrolPath.BP_PatrolPath_C|GetCheckpoints _patrolpath))
  (if (not (Math|Boolean|ORBoolean (Variables|GuardAI|GetbIsChasing) (Variables|GuardAI|GetbIsHalted) (Variables|GuardAI|GetbIsSearching)))
    (if (Utilities|IsValid _patrolpath)
      (if (Utilities|Array|IsValidIndex _checkpoints _checkpointindex)
        (AI|Navigation|MovetoLocation (Math|Transform|TransformLocation (Transformation|GetActorTransform _patrolpath) (Utilities|Array|Get(acopy) _checkpoints _checkpointindex)) 5e+01 true true false true 0)))))

(event Custom|StartChase
  (if (not (Variables|GuardAI|GetbIsHalted))
    (Variables|GuardAI|SetbIsChasing true)
    (Variables|GuardAI|SetbIsSearching false)
    (Default|EnterChase (Variables|GuardAI|GetGuard))
    (AI|Navigation|MovetoActor (Variables|GuardAI|GetChaseTarget) 5.0 true true true 0)))

(event Custom|LoseTarget
  (Variables|GuardAI|SetbIsChasing false)
  (Variables|GuardAI|SetbIsSearching true)
  (Default|EnterSearch (Variables|GuardAI|GetGuard))
  (AI|Navigation|MovetoLocation (Variables|GuardAI|GetLastKnownLocation) 5e+01 true true false true 0))

(event Custom|HandleGameOver
  (Variables|GuardAI|SetbIsHalted true)
  (AI|Navigation|StopMovement))

(event Custom|ReceiveMoveCompleted_Événement
  (params (RequestID :type AI%20Request%20ID%20Structure) (Result :type EPathFollowingResult%20Enum :default "Success"))
  (bind _guard (Variables|GuardAI|GetGuard))
  (if (Variables|GuardAI|GetbIsChasing)
    (Utilities|FlowControl|Delay 0.25)
    (if (Variables|GuardAI|GetbIsChasing)
      (CallFunction|StartChase))
    (elif (Variables|GuardAI|GetbIsSearching)
      (switch Utilities|FlowControl|Switch|SwitchonEPathFollowingResult Result
        (:Success
          _)
        (:Blocked
          _)
        (:OffPath
          _)
        (:Invalid
          _))
      (Utilities|FlowControl|RetriggerableDelay (Variables|/Game/Guards/Characters/BP_Guard.BP_Guard_C|GetSearchDuration (Variables|GuardAI|GetGuard)))
      (CallFunction|FinishSearch)
      (else
        (switch Utilities|FlowControl|Switch|SwitchonEPathFollowingResult Result
          (:Success
            (Variables|GuardAI|SetCheckpointIndex (Math|Integer|%(Integer) (+ (Variables|GuardAI|GetCheckpointIndex) 1) (Utilities|Array|Length (Variables|/Game/Guards/Gameplay/BP_PatrolPath.BP_PatrolPath_C|GetCheckpoints (Variables|/Game/Guards/Characters/BP_Guard.BP_Guard_C|GetPatrolPath _guard)))))
            (Utilities|FlowControl|Delay (Variables|/Game/Guards/Characters/BP_Guard.BP_Guard_C|GetWaitTimeAtCheckpoint _guard))
            (CallFunction|MovetoCurrentCheckpoint))
          (:Blocked
            (Utilities|FlowControl|Delay 1.0 :!label _label)
            (CallFunction|MovetoCurrentCheckpoint))
          (:OffPath
            (goto _label))
          (:Invalid
            (goto _label)))))))

(event Custom|FinishSearch
  (if (Variables|GuardAI|GetbIsSearching)
    (Variables|GuardAI|SetbIsSearching false)
    (Default|EnterPassive (Variables|GuardAI|GetGuard))
    (CallFunction|MovetoCurrentCheckpoint)))

(event EventPossess
  (params (PossessedPawn :type Pawn%20Object%20Reference))
  (bind _asbp_guard (Utilities|Casting|CastToBP_Guard PossessedPawn))
  (Variables|GuardAI|SetGuard _asbp_guard)
  (bind _asbp_guard_game_mode (Utilities|Casting|CastToBP_GuardGameMode (Game|GetGameMode))
    (:then
      (EventDispatchers|BindEventtoOnGameOver _asbp_guard_game_mode (EventDispatchers|CreateEvent :!event Custom|HandleGameOver)))
    (:CastFailed
      _))
  (EventDispatchers|AssignReceiveMoveCompleted (delegate Custom|ReceiveMoveCompleted_Événement))
  (Default|EnterPassive (Variables|GuardAI|GetGuard))
  (CallFunction|MovetoCurrentCheckpoint))

(fn ConstructionScript)